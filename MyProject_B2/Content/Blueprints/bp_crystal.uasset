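; Collectible crystal actor that flies into the player and vanishes when the player pawn overlaps it.
; On overlap it caches its location, scale and point light intensity, then plays a timeline with separate alpha tracks for each.
; The timeline lerps it toward the player's live position while shrinking it to zero and fading the light, then destroys it.
; The pickup is purely visual, with no score or inventory update.
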(event Collision|EventActorBeginOverlap
  (params (OtherActor :type Actor%20Object%20Reference))
  (if (== OtherActor (Game|Player|GetPlayerPawn 0))
    (Variables|Default|SetCryStalLoction (Transformation|GetActorLocation))
    (Variables|Default|SetStartScale (Transformation|GetActorScale3D))
    (Variables|Default|SetStartIntensity (Variables|/Script/Engine.LightComponentBase|GetIntensity (Variables|Default|GetPointLight)))
    (bind (_direction _locationalph _scalealpha _intensityalpha) (Timeline|CollectTimeLine Play)
      (:Update
        (Transformation|SetActorLocation (Math|Vector|Lerp(Vector) (Variables|Default|GetCryStalLoction) (Transformation|GetActorLocation (Game|Player|GetPlayerPawn 0)) _locationalph) false false)
        (Transformation|SetActorScale3D (Math|Vector|Lerp(Vector) (Variables|Default|GetStartScale) "0, 0, 0" _scalealpha))
        (Rendering|Components|Light|SetIntensity (Variables|Default|GetPointLight) (Math|Float|Lerp (Variables|Default|GetStartIntensity) 0.0 _intensityalpha)))
      (:Finished
        (Actor|DestroyActor)))))

(fn ConstructionScript)