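; Torch actor that moves when the player pawn overlaps it.
; The overlap caches the starting location and plays the TorqueMoveLine timeline, adding its vector track to that location as an offset.
; When that finishes, it caches the new position and plays a second timeline to offset the torch from there.
; Both stages move the actor with swept SetActorLocation calls.
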(event Collision|EventActorBeginOverlap
  (params (OtherActor :type Actor%20Object%20Reference))
  (if (== OtherActor (Game|Player|GetPlayerPawn 0))
    (Variables|Default|SetStartLocaton (Transformation|GetActorLocation))
    (bind _vectorlerp (Timeline|TorqueMoveLine PlayFromStart)
      (:Update
        (Transformation|SetActorLocation (+ _vectorlerp (Variables|Default|GetStartLocaton)) true false))
      (:Finished
        (Variables|Default|SetSPos (Transformation|GetActorLocation))
        (bind _vectorlerp_2 (Timeline|Timeline_0 PlayFromStart)
          (:Update
            (Transformation|SetActorLocation (+ _vectorlerp_2 (Variables|Default|GetSPos)) true false)))))))

(fn ConstructionScript)