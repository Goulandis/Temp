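; Cannon actor that automatically and repeatedly fires projectiles from the moment play begins.
; Each cycle waits a short random delay, activates a particle effect and spawns a scaled-down Bp_projectiles at the Arrow component's location and rotation.
; A timeline then slides the Cannon component along its local Y axis, and its event track loops back to the delay for the next shot.
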(event EventBeginPlay
  (bind _arrow (Variables|Default|GetArrow))
  (Utilities|FlowControl|Delay (Math|Random|RandomFloatinRange 0.3 1.0) :!label _label)
  (Components|Activation|Activate (Variables|Default|GetParticle) true)
  (Game|SpawnActorfromClass "/Game/Blueprints/bp_projectiles.bp_projectiles_C" (Math|Transform|MakeTransform (Transformation|GetWorldLocation _arrow) (Transformation|GetWorldRotation _arrow) "0.100000,0.100000,0.100000") "Undefined" 0 0)
  (bind _cannonmove (Timeline|FireTimeLine PlayFromStart)
    (:Update
      (Transformation|SetRelativeLocation (Variables|Default|GetCannon) (Math|Vector|MakeVector 0.0 _cannonmove 0.0) false false))
    (:FileEvent
      (goto _label))))

(fn ConstructionScript)